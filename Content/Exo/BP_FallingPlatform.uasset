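; Falling platform for an exercise (Exo 8) that drops after being hit, then resets itself.
; A component hit from any actor other than player pawn 0 starts a two-second delay, then enables physics simulation on the plank mesh.
; Three seconds later, physics turns off and the mesh returns to the transform saved at BeginPlay.
; A Falling flag, set only after the first delay, blocks retriggers during the fall.
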(event `self.ReceiveBeginPlay`
  (set `self.OriginTransform` (`SceneComponent.K2_GetComponentToWorld` (`self.Pl_woodPlat_2m`))))

(event `self.Pl_woodPlat_2m.OnComponentHit`
  (params (HitComponent :type "PrimitiveComponent Object Reference") (OtherActor :type "Actor Object Reference") (OtherComp :type "PrimitiveComponent Object Reference") (NormalImpulse :type "Vector Structure") (Hit :type "HitResult Structure (by ref)"))
  ;[0.0136 0 0.03125] Exo 8
  (if (!= OtherActor (`GameplayStatics.GetPlayerPawn` 0))
    (if (not (`self.Falling`))
      (`KismetSystemLibrary.Delay` 2.0)
      (set `self.Falling` true)
      (`PrimitiveComponent.SetSimulatePhysics` (`self.Pl_woodPlat_2m`) true)
      (`KismetSystemLibrary.Delay` 3.0)
      (`PrimitiveComponent.SetSimulatePhysics` (`self.Pl_woodPlat_2m`) false)
      (`SceneComponent.K2_SetWorldTransform` (`self.Pl_woodPlat_2m`) (`self.OriginTransform`) false false)
      (set `self.Falling` false))))

(fn `UserConstructionScript`)