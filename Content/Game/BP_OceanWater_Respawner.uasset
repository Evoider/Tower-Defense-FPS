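; Ocean water volume that returns the player to a respawn point on contact and destroys enemies that hit it.
; BeginPlay caches the player character, every TargetPoint in the level as a respawn candidate, and the PlayerStart.
; When the player hits the mesh, a linear scan picks the nearest TargetPoint and teleports them there, falling back to PlayerStart if none is valid.
; Any BP_Enemy that hits it is destroyed.
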(event `self.ReceiveBeginPlay`
  ;[0.2777 0.3166 1] Get RespawnerPoint
  (set `self.PlayerRef` (`GameplayStatics.GetPlayerCharacter` 0))
  (bind _outactors (`GameplayStatics.GetAllActorsOfClass` "/Script/Engine.TargetPoint"))
  (set `self.AllRespanwerPoint` _outactors)
  (bind _returnvalue (`GameplayStatics.GetActorOfClass` "/Script/Engine.PlayerStart"))
  (set `self.PlayerStart` _returnvalue))

(event `self.StaticMeshComponent.OnComponentHit`
  (params (HitComponent :type "PrimitiveComponent Object Reference") (OtherActor :type "Actor Object Reference") (OtherComp :type "PrimitiveComponent Object Reference") (NormalImpulse :type "Vector Structure") (Hit :type "HitResult Structure (by ref)"))
  ;[0.2451 0.648 1] Handle collision &teleportation
  (if (== OtherActor (`self.PlayerRef`))
    (for (_array_element _array_index) (`self.AllRespanwerPoint`)
      (if (== _array_index 0)
        (bind _output_get (set `self.RespawnerPoint` _array_element))
        (else
          (bind _output_get_2 (set `self.temp` _array_element))
          (if (not (< (`self.GetDistanceTo` _output_get (`self.PlayerRef`)) (`self.GetDistanceTo` _output_get_2 (`self.PlayerRef`))))
            (set `self.RespawnerPoint` (`self.temp`))))))
    (bind _respawnerpoint (`self.RespawnerPoint`)
      (:`then`
        (`self.K2_TeleportTo` :`self` (`self.PlayerRef`) :`DestLocation` (`self.K2_GetActorLocation` _respawnerpoint)))
      (:`else`
        (bind _playerstart (`self.PlayerStart`)
          (:`then`
            (`self.K2_TeleportTo` :`self` (`self.PlayerRef`) :`DestLocation` (`self.K2_GetActorLocation` _playerstart)))
          (:`else`))))
    (else
      (bind _asbp_enemy (cast `/Game/Game/Enemy/BP_Enemy` OtherActor))
      (`self.K2_DestroyActor` _asbp_enemy))))

(fn `UserConstructionScript`)