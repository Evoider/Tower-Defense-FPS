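; Defensive tower that automatically fires physics projectiles at enemies and can be destroyed by damage not instigated by the player.
; A detection sphere maintains the enemy set, and a looping timer launches impulse-driven projectiles at its first living entry, adding lift for distant targets.
; Damage updates a camera-facing health bar.
; On death it spawns a portal, deals radial explosion damage, notifies GM_Game and destroys itself.
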(event `self.ReceiveBeginPlay`
  (`|ExecutionSequence`
    (:`then_0`
      (set `self.HealthPoint` (`self.MaxHealthPoint`)))
    (:`then_1`
      (`self.UpdateHealthBar`))
    (:`then_2`
      (`KismetSystemLibrary.K2_SetTimerDelegate` (delegate `TryShoot`) (/ 1.0 (`self.ShootingRate`)) true))))

(event `TryShoot`
  ;[1 1 1] Try to shoot at enemies in range
  (`self.TryToShoot`))

(event `self.ReceiveAnyDamage`
  (params (Damage :type "Float (single-precision)") (DamageType :type "DamageType Object Reference") (InstigatedBy :type "Controller Object Reference") (DamageCauser :type "Actor Object Reference"))
  ;[1 1 1] Take damage
  (if (!= InstigatedBy (`GameplayStatics.GetPlayerController` 0))
    (`self.TakeDamage` Damage)))

(event `self.ReceiveTick`
  (params (DeltaSeconds :type "Float (single-precision)"))
  ;[1 1 1] Rotate HealthBar toward player
  (`SceneComponent.K2_SetWorldRotation` (`self.HealthBar Widget`) (`KismetMathLibrary.Conv_VectorToRotator` (`KismetMathLibrary.GetDirectionUnitVector` (`SceneComponent.K2_GetComponentLocation` (`self.HealthBar Widget`)) (`self.K2_GetActorLocation` (`GameplayStatics.GetPlayerCameraManager` 0)))) false false))

(event `self.SphereDetection.OnComponentBeginOverlap`
  (params (OverlappedComponent :type "PrimitiveComponent Object Reference") (OtherActor :type "Actor Object Reference") (OtherComp :type "PrimitiveComponent Object Reference") (OtherBodyIndex :type Integer) (bFromSweep :type Boolean) (SweepResult :type "HitResult Structure (by ref)"))
  ;[1 1 1] Detect enemy entering shoot range
  (bind _asbp_enemy (cast `/Game/Game/Enemy/BP_Enemy` OtherActor))
  (`BlueprintSetLibrary.Set_Add` (`self.EnemyList`) _asbp_enemy))

(event `self.SphereDetection.OnComponentEndOverlap`
  (params (OverlappedComponent :type "PrimitiveComponent Object Reference") (OtherActor :type "Actor Object Reference") (OtherComp :type "PrimitiveComponent Object Reference") (OtherBodyIndex :type Integer))
  ;[1 1 1] Detect enemy leaving shoot range
  (bind _asbp_enemy (cast `/Game/Game/Enemy/BP_Enemy` OtherActor))
  (`BlueprintSetLibrary.Set_Remove` (`self.EnemyList`) _asbp_enemy))

(event `OnTowerDestroyed`
  ;[1 1 1] Tower destroyed
  (bind _asgm_game (cast `/Game/Game/GameMode/GM_Game` (`GameplayStatics.GetGameMode`)))
  (`/Game/Game/GameMode/GM_Game.OnTowerDestroyed` _asgm_game self)
  (`self.K2_DestroyActor`))

(fn `OnDeath`
  (bind _returnvalue (`self.K2_GetActorLocation`))
  (bind _returnvalue_2 (`SceneComponent.K2_GetComponentLocation` (`self.EffectsLocation`)))
  (`|SpawnActorFromClass` "/Game/Stylized_VFX_StPack/Blueprints/UPDATE_1_2/BP_Portal.BP_Portal_C" (`KismetMathLibrary.MakeTransform` _returnvalue_2 (struct) (* (`KismetMathLibrary.Vector_One`) 3.0)) "Undefined" "MultiplyWithRoot" null false 5.0 null)
  (`GameplayStatics.SpawnSoundAtLocation` "/Game/StarterContent/Audio/Explosion01.Explosion01" _returnvalue_2 (struct) 1.0 1.0 0.0 null null)
  (`GameplayStatics.ApplyRadialDamage` (`self.Death Base Damage`) _returnvalue (`self.Death Damage Radius`) null (`|MakeArray` self :!type "Actor Object Reference") null null)
  (`NiagaraFunctionLibrary.SpawnSystemAtLocation` "/Game/Stylized_VFX_StPack/Particles/UPDATE_1_4/P_Shockwave_Expl_03.P_Shockwave_Expl_03" _returnvalue (struct) (5.0 5.0 5.0))
  (`self.OnTowerDestroyed`))

(fn `TakeDamage`
  (params (Damage :type "Float (double-precision)"))
  (set `self.HealthPoint` (`KismetMathLibrary.FClamp` (- (`self.HealthPoint`) Damage) 0.0 (`self.MaxHealthPoint`)))
  (`self.UpdateHealthBar`)
  (`|SpawnActorFromClass` "/Game/Game/Tower/BP_TowerExplosionHit.BP_TowerExplosionHit_C" (`KismetMathLibrary.MakeTransform` (`SceneComponent.K2_GetComponentLocation` (`self.EffectsLocation`)) (struct) (* (`KismetMathLibrary.Vector_One`) 2.0)) "Undefined" "MultiplyWithRoot" null null)
  (if (<= (`self.HealthPoint`) 0.0)
    (`self.OnDeath`)))

(fn `TryToShoot`
  (bind _returnvalue (`SceneComponent.K2_GetComponentLocation` (`self.ShootLocation`)))
  (if (`BlueprintSetLibrary.Set_IsNotEmpty` (`self.EnemyList`))
    (bind _result (`BlueprintSetLibrary.Set_ToArray` (`self.EnemyList`)))
    (bind _output (`|GetArrayItem` _result))
    (if (`/Game/Game/Enemy/BP_Enemy.IsDead` _output)
      (`BlueprintSetLibrary.Set_Remove` (`self.EnemyList`) _output)
      (`self.TryShoot`)
      (else
        (bind _returnvalue_2 (`|SpawnActorFromClass` "/Game/Game/Tower/BP_TowerProjectile.BP_TowerProjectile_C" (`KismetMathLibrary.MakeTransform` _returnvalue) "AdjustIfPossibleButAlwaysSpawn" "MultiplyWithRoot" null null))
        (`GameplayStatics.SpawnSoundAtLocation` "/Game/Game/Sounds/SC_BlastTower.SC_BlastTower" _returnvalue (struct) 1.0 1.0 0.0 null null)
        (set `/Game/Game/Tower/BP_TowerProjectile.Damages` (`self.Damages`) _returnvalue_2)
        (if (< (`self.GetDistanceTo` _output) 500.0)
          (bind _staticmesh (`/Game/Game/Tower/BP_TowerProjectile.StaticMesh` _returnvalue_2))
          (bind _returnvalue_3 (* (`KismetMathLibrary.GetDirectionUnitVector` _returnvalue (`self.K2_GetActorLocation` _output)) (`self.ImpulseForce`)))
          (`PrimitiveComponent.AddImpulse` _staticmesh _returnvalue_3 "None" false)
          (else
            (`PrimitiveComponent.AddImpulse` _staticmesh (`KismetMathLibrary.MakeVector` (.x _returnvalue_3) (.y _returnvalue_3) (+ (.z _returnvalue_3) 1000.0)) "None" false)))))))

(fn `UpdateHealthBar`
  (bind _aswbp_health_bar (cast `/Game/Game/UI/WBP_HealthBar` (`WidgetComponent.GetWidget` (`self.HealthBar Widget`))))
  (`ProgressBar.SetPercent` (`/Game/Game/UI/WBP_HealthBar.HealthBar` _aswbp_health_bar) (/ (`self.HealthPoint`) (`self.MaxHealthPoint`))))

(fn `UserConstructionScript`
  (`SphereComponent.SetSphereRadius` (`self.SphereDetection`) (`self.ShootingRadius`) true))