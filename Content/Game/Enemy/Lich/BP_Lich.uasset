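; Lich enemy Blueprint that attacks towers, extending a parent class's setup and activating movement on BeginPlay.
; Attack stops active movement and sets the attacking flag.
; DealDamages applies BaseDamage to a valid TargetTower, clears the flag and returns the tower; its multiplier is defaulted but never applied.
; AddEffectToHands attaches a Niagara spell effect to both hand sockets, tinted through a named color parameter.
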(event `self.ReceiveBeginPlay`
  (`parent.ReceiveBeginPlay`)
  (`self.ActivateMovement`))

(event `/Game/Game/Enemy/AI/BPI_AIEnemy.Attack`
  (`NavMovementComponent.StopActiveMovement` (`self.CharacterMovement`))
  (set `self.IsAttacking` true))

(fn `AddEffectToHands`
  (params (Effet :type "NiagaraSystem Object Reference") (Color :type "LinearColor Structure") (ColorParamName :type Name))
  (locals (Effect :type "NiagaraSystem Object Reference" :default "/Script/Niagara.NiagaraSystem'/Game/Stylized_VFX_StPack/Particles/UPDATE_1_2/P_Classic_Hit_02.P_Classic_Hit_02'") (ColorParameterName :type Name :default "None") (SpellColor :type "LinearColor Structure"))
  (bind _output_get (set `local.Effect` Effet))
  (set `local.ColorParameterName` ColorParamName)
  (set `local.SpellColor` Color)
  (bind _returnvalue (`NiagaraFunctionLibrary.SpawnSystemAttached` _output_get (`self.Mesh`) "RightHand" (0.0 0.0 0.0) (struct) "SnapToTarget" true))
  (set `self.RightHandEffect` _returnvalue)
  (bind _returnvalue_2 (`NiagaraFunctionLibrary.SpawnSystemAttached` (`local.Effect`) (`self.Mesh`) "LeftHand" (0.0 0.0 0.0) (struct) "SnapToTarget" true))
  (set `self.LeftHandEffect` _returnvalue_2)
  (`NiagaraComponent.SetVariableLinearColor` (`self.RightHandEffect`) (`local.ColorParameterName`) (`local.SpellColor`))
  (`NiagaraComponent.SetVariableLinearColor` (`self.LeftHandEffect`) (`local.ColorParameterName`) (`local.SpellColor`)))

(fn `DealDamages`
  (params (`Multiplly by` :type "Float (double-precision)"))
  (returns (Target :type "/Game/Game/Tower/BP_Tower Object Reference"))
  (locals (Multiplicator :type "Float (double-precision)"))
  (bind _output_get (set `local.Multiplicator` `Multiplly by`))
  (if (not (!= _output_get 0.0))
    (set `local.Multiplicator` 1.0))
  (bind _targettower (`self.TargetTower`)
    (:`then`
      (`GameplayStatics.ApplyDamage` _targettower (`self.Base Damage`) (`self.GetController`) self)
      (set `self.IsAttacking` false)
      (return (`self.TargetTower`)))
    (:`else`)))

(fn `UserConstructionScript`
  (`parent.UserConstructionScript`))