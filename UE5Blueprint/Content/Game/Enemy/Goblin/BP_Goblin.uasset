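; BP_Goblin is a goblin enemy Blueprint that attacks a target tower and relies on its parent class for begin play and overlap handling.
; Its Attack event stops active movement and sets an attacking flag.
; DealDamage applies base damage to the target tower and clears that flag.
; The Tick event is disabled.
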(event `self.ReceiveBeginPlay`
  (`parent.ReceiveBeginPlay`))

(event `self.ReceiveActorBeginOverlap`
  (params (OtherActor :type "Actor Object Reference"))
  (`parent.ReceiveActorBeginOverlap` OtherActor))

(event `/Game/Game/Enemy/AI/BPI_AIEnemy.Attack`
  ;[0.3646 0.1862 0.4583] Handle attack
  (`NavMovementComponent.StopActiveMovement` (`self.CharacterMovement`))
  (set `self.IsAttacking` true))

(event `DealDamage`
  ;[0.5167 0.574 1] Handle Damage
  (`GameplayStatics.ApplyDamage` (`self.TargetTower`) (`self.Base Damage`))
  (set `self.IsAttacking` false))

(fn `UserConstructionScript`
  (`parent.UserConstructionScript`))