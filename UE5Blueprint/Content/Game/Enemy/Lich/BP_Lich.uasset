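; BP_Lich is an enemy Blueprint for a lich that attacks a target tower.
; On BeginPlay it calls the parent logic, then sets its idle-walk blend space and right-hand attack montage.
; Attack stops active movement and plays the montage, applying base damage to the target tower when the montage's "Hit" notify begins.
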(event `self.ReceiveBeginPlay`
  (`parent.ReceiveBeginPlay`)
  (set `self.BlendSpaceMovement` "/Game/Game/Enemy/Lich/Animations/BSPS_Lich_Idle_Walk.BSPS_Lich_Idle_Walk")
  (set `self.AttackAnimMontage` "/Game/Game/Enemy/Lich/Animations/AM_Lich_Attack_Right_Montage.AM_Lich_Attack_Right_Montage"))

(event `/Game/Game/Enemy/AI/BPI_AIEnemy.Attack`
  (`NavMovementComponent.StopActiveMovement` (`self.CharacterMovement`))
  (bind _notifyname (`|PlayMontage` (`self.Mesh`) (`self.AttackAnimMontage`))
    (:`OnNotifyBegin`
      (if (== _notifyname "Hit")
        (`GameplayStatics.ApplyDamage` (`self.TargetTower`) (`self.Base Damage`))))))

(fn `UserConstructionScript`
  (`parent.UserConstructionScript`))