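; Enemy character that walks to a random tower from GM_Game's list and attacks it.
; A self-repeating loop uses AI MoveTo, attacks once in range, waits, then picks another tower if the target is gone.
; Damage updates a camera-facing health bar and briefly flags a hit; zero life stops movement and relaxes collision, with destruction in a separate Die function.
; Nav mesh jumps launch the character along a suggested projectile arc.
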(event `self.ReceiveBeginPlay`
  (`|ExecutionSequence`
    (:`then_0`
      (set `self.Life` (`self.MaxLife`))
      (`self.UpdateHealthBar`))
    (:`then_1`
      (`self.SetTargetTower`)
      (`self.MoveToTower`))))

(event `self.ReceiveTick`
  (params (DeltaSeconds :type "Float (single-precision)"))
  ;[0.004506 0 0.01042] Update Healthbar rotation toward player
  (`SceneComponent.K2_SetWorldRotation` (`self.HealthBar Widget`) (`KismetMathLibrary.Conv_VectorToRotator` (`KismetMathLibrary.GetDirectionUnitVector` (`SceneComponent.K2_GetComponentLocation` (`self.HealthBar Widget`)) (`self.K2_GetActorLocation` (`GameplayStatics.GetPlayerCameraManager` 0)))) false false))

(event `self.ReceiveAnyDamage`
  (params (Damage :type "Float (single-precision)") (DamageType :type "DamageType Object Reference") (InstigatedBy :type "Controller Object Reference") (DamageCauser :type "Actor Object Reference"))
  ;[0.004506 0 0.01042] Get Hurt
  (`self.UpdateLife` Damage)
  (set `self.IsHit` true)
  (`KismetSystemLibrary.Delay` 0.1)
  (set `self.IsHit` false))

(event `MoveToTower`
  (bind _attackingrange (`self.AttackingRange`))
  ;[1 1 1] Go To Tower or Attack
  (if (not (`self.IsDead`))
    (bind _targettower (`self.TargetTower`)
      (:`then`
        (if (<= (`self.GetDistanceTo` _targettower) _attackingrange)
          (`/Game/Game/Enemy/AI/BPI_AIEnemy.Attack` :!label _label)
          (`KismetSystemLibrary.Delay` 1.0)
          (`self.TargetTower`
            (:`then`
              _)
            (:`else`
              (`self.GetTargetTower` :!label _label_2)))
          (else
            (`|AIMoveTo` self (0.0 0.0 0.0) _targettower _attackingrange true
              (:`OnSuccess`
                (`self.K2_SetActorRotation` (`KismetMathLibrary.Conv_VectorToRotator` (`KismetMathLibrary.GetDirectionUnitVector` (`self.K2_GetActorLocation`) (`self.K2_GetActorLocation` (`self.TargetTower`)))))
                (goto _label))
              (:`OnFail`
                (goto _label_2)))))
        (`self.MoveToTower`))
      (:`else`))))

(event `/Game/Game/Enemy/AI/BPI_AIEnemy.JumpToDestination`
  (params (Destination :type "Vector Structure"))
  ;[1 1 1] Jump nav mesh
  (bind _outlaunchvelocity (`GameplayStatics.SuggestProjectileVelocity_CustomArc` (`self.K2_GetActorLocation`) (`KismetMathLibrary.MakeVector` (.x Destination) (.y Destination) (+ (.z Destination) 350.0))))
  (`self.LaunchCharacter` _outlaunchvelocity true true))

(fn `DeactivateCollision`
  (`PrimitiveComponent.SetCollisionResponseToChannel` (`self.CapsuleComponent`) "ECC_GameTraceChannel1" "ECR_Ignore")
  (`PrimitiveComponent.SetCollisionResponseToChannel` (`self.Mesh`) "ECC_WorldStatic" "ECR_Ignore")
  (`PrimitiveComponent.SetCollisionResponseToChannel` (`self.CapsuleComponent`) "ECC_Pawn" "ECR_Ignore")
  (`PrimitiveComponent.SetCollisionResponseToChannel` (`self.Mesh`) "ECC_Pawn" "ECR_Ignore"))

(fn `Die`
  (`self.DetachFromControllerPendingDestroy`)
  (`self.K2_DestroyActor`)
  (`self.On Destroyed`))

(fn `GetTargetTower`
  (returns (TargetTower :type "/Game/Game/Tower/BP_Tower Object Reference"))
  (bind _targettower (`self.TargetTower`)
    (:`then`
      (return _targettower))
    (:`else`
      (`self.SetTargetTower`)
      (return null))))

(fn `SetTargetTower`
  (bind _asgm_game (cast `/Game/Game/GameMode/GM_Game` (`GameplayStatics.GetGameMode`)))
  (set `self.TargetTower` (`KismetArrayLibrary.Array_Random` (`/Game/Game/GameMode/GM_Game.Towers` _asgm_game))))

(fn `UpdateHealthBar`
  (bind _aswbp_health_bar (cast `/Game/Game/WBP_HealthBar` (`WidgetComponent.GetWidget` (`self.HealthBar Widget`))))
  (`ProgressBar.SetPercent` (`/Game/Game/WBP_HealthBar.HealthBar` _aswbp_health_bar) (/ (`self.Life`) (`self.MaxLife`))))

(fn `UpdateLife`
  (params (Value :type "Float (double-precision)"))
  (bind _output_get (set `self.Life` (- (`self.Life`) Value)))
  (`self.UpdateHealthBar`)
  (if (<= _output_get 0.0)
    (set `self.IsDead` true)
    (`NavMovementComponent.StopActiveMovement` (`self.CharacterMovement`))
    (`self.DeactivateCollision`)))

(fn `UserConstructionScript`)