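; BP_Enemy1 is an enemy pawn that walks toward the tower and dies when damage depletes its life.
; On BeginPlay, GoToTower finds the BP_Tower actor and uses AI MoveTo to approach it, re-issuing the move after a short delay only on success.
; AnyDamage subtracts from Life and, at zero or below, destroys the actor and then calls the OnDestroyed dispatcher.
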(event `self.ReceiveBeginPlay`
  (`self.GoToTower`))

(event `GoToTower`
  (bind _returnvalue (`GameplayStatics.GetActorOfClass` "/Game/Game/Tower/BP_Tower.BP_Tower_C"))
  (`|AIMoveTo` self (0.0 0.0 0.0) _returnvalue 500.0
    (:`OnSuccess`
      (`KismetSystemLibrary.Delay` 2.0)
      (`self.GoToTower`))))

(event `self.ReceiveAnyDamage`
  (params (Damage :type "Float (single-precision)") (DamageType :type "DamageType Object Reference") (InstigatedBy :type "Controller Object Reference") (DamageCauser :type "Actor Object Reference"))
  (bind _output_get (set `self.Life` (- (`self.Life`) Damage)))
  (if (<= _output_get 0.0)
    (`self.K2_DestroyActor`)
    (`self.On Destroyed`)))

(fn `UserConstructionScript`)