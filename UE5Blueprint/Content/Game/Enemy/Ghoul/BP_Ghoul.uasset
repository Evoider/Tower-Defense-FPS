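; BP_Ghoul is a ghoul enemy that attacks a target tower.
; Attack stops active movement and sets an attacking flag, while DealDamage applies base damage to the tower and clears that flag.
; BeginPlay, Tick, overlap and construction logic only forward to the parent class.
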(event `self.ReceiveBeginPlay`
  (`parent.ReceiveBeginPlay`))

(event `self.ReceiveTick`
  (params (DeltaSeconds :type "Float (single-precision)"))
  (`parent.ReceiveTick` DeltaSeconds))

(event `self.ReceiveActorBeginOverlap`
  (params (OtherActor :type "Actor Object Reference"))
  (`parent.ReceiveActorBeginOverlap` OtherActor))

(event `/Game/Game/Enemy/AI/BPI_AIEnemy.Attack`
  ;[1 1 1] Attack
  (`NavMovementComponent.StopActiveMovement` (`self.CharacterMovement`))
  (set `self.IsAttacking` true))

(event `DealDamage`
  ;[1 1 1] Damage
  (`GameplayStatics.ApplyDamage` (`self.TargetTower`) (`self.Base Damage`))
  (set `self.IsAttacking` false))

(fn `UserConstructionScript`
  (`parent.UserConstructionScript`))