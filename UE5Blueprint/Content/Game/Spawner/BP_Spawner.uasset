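; BP_Spawner is an enemy spawner that releases queued enemy classes at its spawn point and reports their destruction to GM_Game.
; After a startup delay, a looping timer spawns the next queued enemy while IsOn, and hides the spawner otherwise.
; AddEnemyToQueue also tries an immediate spawn when no BP_Enemy overlaps its sphere.
; The game mode's end-game event switches the spawner off and requests clearing the timer.
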(event `self.ReceiveBeginPlay`
  (`KismetSystemLibrary.Delay` 3.0)
  (`KismetSystemLibrary.K2_SetTimerDelegate` (delegate `TryToSpawn`) 0.5 true)
  (bind _asgm_game (cast `/Game/Game/GameMode/GM_Game` (`GameplayStatics.GetGameMode`)))
  (add `/Game/Game/GameMode/GM_Game.OnEndGame` _asgm_game (delegate `StopSpawning`)))

(event `TryToSpawn`
  (if (`self.IsOn`)
    (`self.SetActorHiddenInGame` false)
    (`self.SpawnEnemy`)
    (else
      (`self.SetActorHiddenInGame` true))))

(event `StopSpawning`
  (params (Win :type Boolean))
  (set `self.IsOn` false)
  (`KismetSystemLibrary.K2_ClearTimer` null "TryToSpawn"))

(event `OnEnemyDefeated`
  (params (DestroyedActor :type "Actor Object Reference"))
  (bind _asgm_game (cast `/Game/Game/GameMode/GM_Game` (`GameplayStatics.GetGameMode`)))
  (`/Game/Game/GameMode/GM_Game.OnEnemyDefeated` _asgm_game))

(fn `AddEnemyToQueue`
  (params (EnemyClass :type "/Game/Game/Enemy/BP_Enemy Class Reference (by ref)"))
  (`KismetArrayLibrary.Array_Add` (`self.EnemyQueue`) EnemyClass)
  (if (not (`KismetArrayLibrary.Array_IsValidIndex` (`PrimitiveComponent.GetOverlappingActors` (`self.Sphere`) "/Game/Game/Enemy/BP_Enemy.BP_Enemy_C")))
    (`self.SpawnEnemy`)))

(fn `SpawnEnemy`
  (returns (Success :type Boolean))
  (if (and (`self.IsOn`) (`KismetArrayLibrary.Array_IsValidIndex` (`self.EnemyQueue`)))
    (bind _returnvalue (`|SpawnActorFromClass` (`|GetArrayItem` (`self.EnemyQueue`)) (`SceneComponent.K2_GetComponentToWorld` (`self.SpawnPoint`)) "AdjustIfPossibleButAlwaysSpawn" "MultiplyWithRoot" null null))
    (add `self.OnDestroyed` _returnvalue (`|CreateDelegate` :!event `OnEnemyDefeated`))
    (`KismetArrayLibrary.Array_Remove` (`self.EnemyQueue`))
    (return true)
    (else
      (return false))))

(fn `UserConstructionScript`)