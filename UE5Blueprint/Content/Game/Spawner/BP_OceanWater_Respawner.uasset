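; Ocean water actor that returns the player to the nearest respawn point when they hit its mesh.
; On BeginPlay it caches the first player character and every TargetPoint actor in the level as candidate respawn points.
; On a hit from that player, it loops through the points to find the closest one, teleports the player there with zero rotation, and logs success or failure.
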(event `self.ReceiveBeginPlay`
  ;[0.2777 0.3166 1] Get RespawnerPoint
  (set `self.PlayerRef` (`GameplayStatics.GetPlayerCharacter` 0))
  (bind _outactors (`GameplayStatics.GetAllActorsOfClass` "/Script/Engine.TargetPoint"))
  (set `self.AllRespanwerPoint` _outactors))

(event `self.StaticMeshComponent.OnComponentHit`
  (params (HitComponent :type "PrimitiveComponent Object Reference") (OtherActor :type "Actor Object Reference") (OtherComp :type "PrimitiveComponent Object Reference") (NormalImpulse :type "Vector Structure") (Hit :type "HitResult Structure (by ref)"))
  ;[0.2451 0.648 1] Handle collision &teleportation
  (if (== OtherActor (`self.PlayerRef`))
    (for (_array_element _array_index) (`self.AllRespanwerPoint`)
      (if (== _array_index 0)
        (bind _output_get (set `self.RespawnerPoint` _array_element))
        (else
          (bind _output_get_2 (set `self.temp` _array_element))
          (if (not (< (`self.GetDistanceTo` _output_get (`self.PlayerRef`)) (`self.GetDistanceTo` _output_get_2 (`self.PlayerRef`))))
            (set `self.RespawnerPoint` (`self.temp`))))))
    (bind _returnvalue (`self.K2_TeleportTo` :`self` (`self.PlayerRef`) :`DestLocation` (`self.K2_GetActorLocation` (`self.RespawnerPoint`))))
    (if _returnvalue
      (`KismetSystemLibrary.PrintString` "Succesfully teleported" false true (struct :`G` 0.66 :`B` 1.0 :`A` 1.0) 5.0)
      (else
        (`KismetSystemLibrary.PrintString` "Couldn't teleport" false true (struct :`G` 0.66 :`B` 1.0 :`A` 1.0) 5.0)))))

(fn `UserConstructionScript`)