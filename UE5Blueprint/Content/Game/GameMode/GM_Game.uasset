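; Game mode for a wave-based tower defense match that runs waves, tracks towers and ends in a loss when none remain.
; Each wave loads an enemy class-count pool from DT_WavePool, queues a capped batch on random active BP_Spawners and refills on kills.
; Clearing a wave starts a timer for the next.
; Towers become targets one group at a time, advancing as groups fall, and event dispatchers broadcast game progress.
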(event `self.ReceiveBeginPlay`
  (bind _returnvalue (`|CreateWidget` "/Game/Game/UI/WBP_WaveModeHUD.WBP_WaveModeHUD_C"))
  (`UserWidget.AddToViewport` _returnvalue 0)
  (`self.SetupGame`)
  (bind _returnvalue_2 (`KismetSystemLibrary.K2_SetTimer` null "NewWave" (`self.TimeBeforeStart`)))
  (set `self.StartTimer` _returnvalue_2)
  (`self.OnStartGame`))

(event `EndGame`
  (params (Win :type Boolean))
  (bind _returnvalue (`|CreateWidget` "/Game/Game/UI/WBP_WinLose.WBP_WinLose_C"))
  (`UserWidget.AddToViewport` _returnvalue 0)
  (`self.OnEndGame` Win))

(fn `ActivateTowers`
  (`self.UpdateCurrentTowerGroup`)
  (for _array_element (`self.TowersAll`)
    (if (`|EnumEquality` (`/Game/Game/Tower/BP_Tower.TowerGroup` _array_element) (`self.CurrentTowerGroup`))
      (set `/Game/Game/Tower/BP_Tower.IsTarget` true _array_element)
      (`KismetSystemLibrary.PrintString` "Hello" true true (struct :`R` 1.0 :`A` 1.0) 10.0)
      (else
        (set `/Game/Game/Tower/BP_Tower.IsTarget` false _array_element)))))

(fn `BuildEnemyPool`
  (locals (Enemy :type "/Game/Game/Enemy/BP_Enemy Class Reference"))
  (bind _returnvalue (`|GetDataTableRow` "/Game/Game/Spawner/DT_WavePool.DT_WavePool" (`KismetStringLibrary.Conv_StringToName` (`KismetStringLibrary.Conv_IntToString` (`self.WaveNumber`))))
    (:`then`
      (set `self.EnemyPool` (`.EnemyPool_5_BFC9750445596842C794E690E4623AC6` (break `/Game/Game/Spawner/STR_Wave` _returnvalue)))
      (set `self.EnemyRemaining` (`self.GetPoolSize`)))))

(fn `EndWave`
  (`self.ActivateTowers`)
  (`self.OnEndWave`))

(fn `EnterTransition`
  (params (TTransitionPeriod :type "Float (single-precision)"))
  (bind _returnvalue (`KismetSystemLibrary.K2_SetTimer` null "NewWave" TTransitionPeriod))
  (set `self.TransitionTimer` _returnvalue)
  (`self.EndWave`))

(fn `GetActiveTowers`
  (locals (LocalTower :type "/Game/Game/Tower/BP_Tower Object Reference") (LocalTowers :type "Array of /Game/Game/Tower/BP_Tower Object Reference"))
  (bind _towerdestrroyed (`self.TowerDestrroyed`))
  (bind _output_get (set `local.LocalTowers` (`self.TowersAll`)))
  (for _array_element _output_get
    (set `local.LocalTower` _array_element)
    (if (and (!= (`self.TowerDestrroyed`) (`local.LocalTower`)) (`/Game/Game/Tower/BP_Tower.IsTarget` (`local.LocalTower`)))
      (`KismetArrayLibrary.Array_AddUnique` (`self.TowersActive`) (`local.LocalTower`))))
  (`KismetArrayLibrary.Array_RemoveItem` (`self.TowersActive`) _towerdestrroyed)
  (`KismetArrayLibrary.Array_RemoveItem` (`self.TowersAll`) _towerdestrroyed)
  (set `self.TowerDestrroyed` null))

(fn `GetAllTowers`
  (returns (Towers :type "Array of /Game/Game/Tower/BP_Tower Object Reference"))
  (bind _outactors (`GameplayStatics.GetAllActorsOfClass` "/Game/Game/Tower/BP_Tower.BP_Tower_C"))
  (bind _output_get (set `self.TowersAll` _outactors))
  (return _output_get))

(fn `GetEnemyFromPool`
  (returns (Enemy :type "/Game/Game/Enemy/BP_Enemy Class Reference"))
  (locals (LocalClassChoice :type "/Game/Game/Enemy/BP_Enemy Class Reference"))
  (bind _enemypool (`self.EnemyPool`))
  (bind _localclasschoice (`local.LocalClassChoice`))
  (bind _localclasschoice_2 (`local.LocalClassChoice`))
  (bind _keys (`BlueprintMapLibrary.Map_Keys` (`self.EnemyPool`)))
  (bind _output_get (set `local.LocalClassChoice` (`KismetArrayLibrary.Array_Random` _keys)))
  (bind _returnvalue (- (`BlueprintMapLibrary.Map_Find` (`self.EnemyPool`) _output_get) 1))
  (if (> _returnvalue 0)
    (`BlueprintMapLibrary.Map_Add` _enemypool _localclasschoice _returnvalue)
    (return _localclasschoice_2)
    (else
      (`BlueprintMapLibrary.Map_Remove` _enemypool _localclasschoice)
      (return _localclasschoice_2))))

(fn `GetPoolSize`
  (returns (Sum :type Integer))
  (locals (LocalSum :type Integer))
  (bind _localsum (`local.LocalSum`))
  (bind _values (`BlueprintMapLibrary.Map_Values` (`self.EnemyPool`)))
  (for _array_element _values
    (set `local.LocalSum` (+ _array_element _localsum)))
  (return _localsum))

(fn `GetSpawners`
  (locals (LocalSpawners :type "Array of /Game/Game/Spawner/BP_Spawner Object Reference"))
  (bind _outactors (`GameplayStatics.GetAllActorsOfClass` "/Game/Game/Spawner/BP_Spawner.BP_Spawner_C"))
  (bind _output_get (set `self.Spawners` _outactors))
  (bind _output_get_2 (set `local.LocalSpawners` _output_get))
  (for _array_element _output_get_2
    (if (not (`/Game/Game/Spawner/BP_Spawner.IsOn` _array_element))
      (`KismetArrayLibrary.Array_RemoveItem` (`self.Spawners`) _array_element))))

(fn `NewWave`
  (bind _wavenumber (`self.WaveNumber`))
  (`/Engine/EditorBlueprintResources/StandardMacros.IncrementInt` _wavenumber
    (:`  `
      (`self.GetActiveTowers`)
      (`self.GetSpawners`)
      (`self.StartWave`)
      (`self.OnNewWave` _wavenumber (`self.EnemyRemaining`) (`self.TowersRemaining`)))))

(fn `OnEnemyDefeated`
  (bind _enemyremaining (`self.EnemyRemaining`))
  (bind _result (`/Engine/EditorBlueprintResources/StandardMacros.DecrementInt` _enemyremaining)
    (:`  `
      (`self.OnEnemyKilled` _enemyremaining)
      (if (< _result (`self.EnemyMaxCount`))
        (if (<= (`self.EnemyRemaining`) 0)
          (`self.EnterTransition` 5.0))
        (else
          (bind _enemy (`self.GetEnemyFromPool`))
          (`/Game/Game/Spawner/BP_Spawner.AddEnemyToQueue` (`KismetArrayLibrary.Array_Random` (`self.Spawners`)) _enemy))))))

(fn `OnTowerDestroyed`
  (params (TowerDestroyed :type "/Game/Game/Tower/BP_Tower Object Reference"))
  (bind _towersremaining (`self.TowersRemaining`))
  (set `self.TowerDestrroyed` TowerDestroyed)
  (`/Engine/EditorBlueprintResources/StandardMacros.DecrementInt` _towersremaining
    (:`  `
      (`self.OnTowerBoom` _towersremaining)
      (`self.ActivateTowers`))))

(fn `SetupGame`
  (`self.GetAllTowers`)
  (set `self.TowersRemaining` (`KismetArrayLibrary.Array_Length` (`self.TowersAll`)))
  (`self.ActivateTowers`))

(fn `StartWave`
  (bind _sum (`self.GetPoolSize`))
  (bind _spawners (`self.Spawners`))
  (bind _returnvalue (/ _sum 4))
  (`self.BuildEnemyPool`)
  (if (== _returnvalue 0)
    (set `self.EnemyMaxCount` (+ _returnvalue 2))
    (else
      (set `self.EnemyMaxCount` _returnvalue)))
  (for _ (range 1 (+ (`KismetMathLibrary.Min` _sum (`self.EnemyMaxCount`)) 1))
    (bind _enemy (`self.GetEnemyFromPool`))
    (if (`KismetArrayLibrary.Array_IsValidIndex` _spawners)
      (`/Game/Game/Spawner/BP_Spawner.AddEnemyToQueue` (`KismetArrayLibrary.Array_Random` _spawners) _enemy))))

(fn `UpdateCurrentTowerGroup`
  (`self.GetActiveTowers`)
  (if (`KismetArrayLibrary.Array_IsValidIndex` (`self.TowersAll`))
    (if (not (`KismetArrayLibrary.Array_IsValidIndex` (`self.TowersActive`)))
      (switch `/Game/Game/Tower/E_TowerGroup` (`self.CurrentTowerGroup`)
        (:`NewEnumerator0`
          (set `self.CurrentTowerGroup` "NewEnumerator1"))
        (:`NewEnumerator1`
          (set `self.CurrentTowerGroup` "NewEnumerator2"))
        (:`NewEnumerator2`
          (set `self.CurrentTowerGroup` "NewEnumerator3"))
        (:`NewEnumerator3`
          (set `self.CurrentTowerGroup` "NewEnumerator4")))
      (`KismetSystemLibrary.PrintString` (`|GetEnumeratorNameAsString` (`self.CurrentTowerGroup`)) true true (struct :`G` 0.66 :`B` 1.0 :`A` 1.0) 10.0))
    (else
      (`self.EndGame` false))))

(fn `UserConstructionScript`)