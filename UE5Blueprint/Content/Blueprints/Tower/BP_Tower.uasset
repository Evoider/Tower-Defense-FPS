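; BP_Tower is an enemy tower that shoots at the player and spawns a portal when destroyed.
; A looping timer checks player distance and, within range, spawns a BP_TowerProjectile and launches it toward the player with a physics impulse.
; AnyDamage lowers clamped health, updates a widget health bar that Tick turns toward the camera, and spawns hit effects.
; The detection sphere overlap only prints a debug message.
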(event `self.ReceiveBeginPlay`
  (`|ExecutionSequence`
    (:`then_0`
      (set `self.HealthPoint` (`self.MaxHealthPoint`)))
    (:`then_1`
      (`self.UpdateHealthBar`))
    (:`then_2`
      (`KismetSystemLibrary.K2_SetTimerDelegate` (delegate `TryShoot`) 2.0 true))))

(event `TryShoot`
  (bind _returnvalue (`GameplayStatics.GetPlayerCharacter` 0))
  (bind _returnvalue_2 (`SceneComponent.K2_GetComponentLocation` (`self.ShootLocation`)))
  (if (<= (`self.GetDistanceTo` _returnvalue) 1000.0)
    (bind _returnvalue_3 (`|SpawnActorFromClass` "/Game/Blueprints/Tower/BP_TowerProjectile.BP_TowerProjectile_C" (`KismetMathLibrary.MakeTransform` _returnvalue_2) "Undefined" "MultiplyWithRoot" null null))
    (set `/Game/Blueprints/Tower/BP_TowerProjectile.Damages` (`self.Damages`) _returnvalue_3)
    (`PrimitiveComponent.AddImpulse` (`/Game/Blueprints/Tower/BP_TowerProjectile.StaticMesh` _returnvalue_3) (* (`KismetMathLibrary.GetDirectionUnitVector` _returnvalue_2 (`self.K2_GetActorLocation` _returnvalue)) (`self.ImpulseForce`)) "None" false)))

(event `self.ReceiveTick`
  (params (DeltaSeconds :type "Float (single-precision)"))
  ;[1 1 1] Rotate HealthBar toward player
  (`SceneComponent.K2_SetWorldRotation` (`self.HealthBar Widget`) (`KismetMathLibrary.Conv_VectorToRotator` (`KismetMathLibrary.GetDirectionUnitVector` (`SceneComponent.K2_GetComponentLocation` (`self.HealthBar Widget`)) (`self.K2_GetActorLocation` (`GameplayStatics.GetPlayerCameraManager` 0)))) false false))

(event `self.ReceiveAnyDamage`
  (params (Damage :type "Float (single-precision)") (DamageType :type "DamageType Object Reference") (InstigatedBy :type "Controller Object Reference") (DamageCauser :type "Actor Object Reference"))
  (bind _returnvalue (`SceneComponent.K2_GetComponentLocation` (`self.EffectsLocation`)))
  ;[1 1 1] Take damage
  (set `self.HealthPoint` (`KismetMathLibrary.FClamp` (- (`self.HealthPoint`) Damage) 0.0 (`self.MaxHealthPoint`)))
  (`self.UpdateHealthBar`)
  (`|SpawnActorFromClass` "/Game/Blueprints/Tower/BP_TowerExplosionHit.BP_TowerExplosionHit_C" (`KismetMathLibrary.MakeTransform` (`SceneComponent.K2_GetComponentLocation` (`self.EffectsLocation`)) (struct) (* (`KismetMathLibrary.Vector_One`) 2.0)) "Undefined" "MultiplyWithRoot" null null)
  (if (<= (`self.HealthPoint`) 0.0)
    (`|SpawnActorFromClass` "/Game/Stylized_VFX_StPack/Blueprints/UPDATE_1_2/BP_Portal.BP_Portal_C" (`KismetMathLibrary.MakeTransform` _returnvalue (struct) (* (`KismetMathLibrary.Vector_One`) 3.0)) "Undefined" "MultiplyWithRoot" null false 5.0 null)
    (`GameplayStatics.SpawnSoundAtLocation` "/Game/StarterContent/Audio/Explosion01.Explosion01" _returnvalue (struct) 1.0 1.0 0.0 null null)
    (`self.K2_DestroyActor`)))

(event `self.SphereDetection.OnComponentBeginOverlap`
  (params (OverlappedComponent :type "PrimitiveComponent Object Reference") (OtherActor :type "Actor Object Reference") (OtherComp :type "PrimitiveComponent Object Reference") (OtherBodyIndex :type Integer) (bFromSweep :type Boolean) (SweepResult :type "HitResult Structure (by ref)"))
  (`KismetSystemLibrary.PrintString` "Hello"))

(fn `UpdateHealthBar`
  (bind _aswbp_health_bar (cast `/Game/Blueprints/WBP_HealthBar` (`WidgetComponent.GetWidget` (`self.HealthBar Widget`))))
  (`ProgressBar.SetPercent` (`/Game/Blueprints/WBP_HealthBar.HealthBar` _aswbp_health_bar) (/ (`self.HealthPoint`) (`self.MaxHealthPoint`))))

(fn `UserConstructionScript`)