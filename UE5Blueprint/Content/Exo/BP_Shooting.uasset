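; BP_Shooting is a turret-style exercise actor (Exo 10) that fires projectiles at the player.
; A Delay on Tick acts as a repeating timer, checking every couple of seconds whether the player pawn is within range.
; When it is, the actor spawns a BP_Cosmic_Projectile at its location, aimed at the player, with gravity off and preset impulse power and level.
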(event `self.ReceiveTick`
  (params (DeltaSeconds :type "Float (single-precision)"))
  (bind _returnvalue (`GameplayStatics.GetPlayerPawn` 0))
  (bind _returnvalue_2 (`self.K2_GetActorLocation`))
  ;[0.0136 0 0.03125] Exo 10
  (`KismetSystemLibrary.Delay` 2.0)
  (if (<= (`self.GetDistanceTo` _returnvalue) 1500.0)
    (`|SpawnActorFromClass` "/Game/Stylized_VFX_StPack/Blueprints/UPDATE_1_2/BP_Cosmic_Projectile.BP_Cosmic_Projectile_C" (`KismetMathLibrary.MakeTransform` _returnvalue_2 (`KismetMathLibrary.Conv_VectorToRotator` (`KismetMathLibrary.GetDirectionUnitVector` _returnvalue_2 (`self.K2_GetActorLocation` _returnvalue)))) "AdjustIfPossibleButAlwaysSpawn" "MultiplyWithRoot" null false 2000.0 2 null)))

(fn `UserConstructionScript`)